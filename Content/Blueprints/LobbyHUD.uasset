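; LobbyHUD is a HUD Blueprint that draws simple text overlays for a lobby screen.
; Each DrawHUD call prints a "Connected:" count of player states in the top-left corner.
; It also draws the CenterText string centred on screen, measuring it with GetTextSize using the configurable font and scale to offset the position.
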(event EventBeginPlay)

(event Collision|EventActorBeginOverlap
  (params (OtherActor :type Actor%20Object%20Reference)))

(event EventTick
  (params (DeltaSeconds :type Float%20%28single-precision%29)))

(event EventDrawHUD
  (params (SizeX :type Integer) (SizeY :type Integer))
  (bind _centertext (Variables|Default|GetCenterText))
  (bind _centertextscale (Variables|Default|GetCenterTextScale))
  (bind _centertextfont (Variables|Default|GetCenterTextFont))
  (bind (_outwidth _outheight) (Class|HUD|GetTextSize _centertext _centertextfont _centertextscale))
  (HUD|DrawText (Utilities|String|Append "Connected: " (Utilities|String|ToString(Integer) (Class|GameplayStatics|GetNumPlayerStates))) "(R=1.000000,G=1.000000,B=1.000000,A=1.000000)" 4e+01 4e+01 "/Engine/EngineFonts/Roboto.Roboto" 1.25 false)
  (HUD|DrawText (Variables|Default|GetCenterText) "(R=1.000000,G=1.000000,B=1.000000,A=1.000000)" (* (- SizeX _outwidth) 0.5) (* (- SizeY _outheight) 0.5) (Variables|Default|GetCenterTextFont) (Variables|Default|GetCenterTextScale) false))

(fn ConstructionScript)