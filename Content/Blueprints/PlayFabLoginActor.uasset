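; Actor that handles PlayFab email and password login and keeps the session in the game instance.
; On BeginPlay it restores the entity token, authentication context and PlayFab ID from PlayFabGameInstance.
; A successful login saves new credentials back there and fires a success event, while the error handler prints and broadcasts the message with its code.
; Helper functions report whether a session is held and extract the entity ID from the token.
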(event Custom|Login%20with%20Email
  (params (Email :type String) (Password :type String))
  (|LoginwithEmailAddress (Utilities|Struct|MakeClientLoginWithEmailAddressRequest 0 Email 0 Password (Variables|Default|GetLoginContext)) (EventDispatchers|CreateEvent :!event LoginSuccessed) (EventDispatchers|CreateEvent :!event PlayfabError)))

(event EventBeginPlay
  (bind _asplay_fab_game_instance (Utilities|Casting|CastToPlayFabGameInstance (Game|GetGameInstance)))
  (Variables|Default|SetLoginEntity (Variables|/Script/PlayFabMultiplayer.PlayFabGameInstance|GetPlayFabLoginEntity _asplay_fab_game_instance))
  (Variables|Default|SetLoginContext (Variables|/Script/PlayFabMultiplayer.PlayFabGameInstance|GetPlayFabLoginContext _asplay_fab_game_instance))
  (Variables|Default|SetPlayFabId (Variables|/Script/PlayFabMultiplayer.PlayFabGameInstance|GetPlayFabMasterId _asplay_fab_game_instance)))

(fn ConstructionScript)

(fn PlayFabError
  (params (error :type Play%20Fab%20Error%20Structure) (customData :type Object%20Object%20Reference))
  (bind (_haserror _errorcode _errorname _errormessage) (Utilities|Struct|BreakPlayFabError error))
  (bind _output_get (LocalVariables|SetMessage (Utilities|String|ToString(Text) (Utilities|Text|FormatText "{Message} ({Code})" _errormessage (Utilities|Text|ToText(Integer) _errorcode false false)))))
  (Development|PrintString _output_get true true "(R=1.000000,G=0.000000,B=0.000000,A=1.000000)")
  (Default|CallOnErrorMessage (LocalVariables|GetMessage)))

(fn IsLoggingin
  (return (and (Utilities|IsValid (Variables|Default|GetLoginEntity)) (Utilities|IsValid (Variables|Default|GetLoginContext)))))

(fn LoginSuccessed
  (params (result :type Client%20Login%20Result%20Structure) (customData :type Object%20Object%20Reference))
  (bind (_entitytoken _inforesultpayload _lastlogintime _newlycreated _playfabid _sessionticket _settingsforuser _treatmentassignment _authenticationcontext) (Utilities|Struct|BreakClientLoginResult result))
  (Variables|Default|SetLoginEntity _entitytoken)
  (Variables|Default|SetPlayFabId _playfabid)
  (Variables|Default|SetLoginContext _authenticationcontext)
  (Utilities|FlowControl|Sequence
    (:then_0
      (bind _asplay_fab_game_instance (Utilities|Casting|CastToPlayFabGameInstance (Game|GetGameInstance)))
      (Class|PlayFabGameInstance|SetPlayFabLoginSession _asplay_fab_game_instance (Variables|Default|GetPlayFabId) (Variables|Default|GetLoginEntity) (Variables|Default|GetLoginContext)))
    (:then_1
      (Default|CallOnLoginSuccessed))))

(fn GetPlayerId
  (bind _loginentity (Variables|Default|GetLoginEntity))
  (if (and (Utilities|IsValid _loginentity) (Class|PlayFabJsonObject|HasField _loginentity "Entity"))
    (return (Class|PlayFabJsonObject|GetStringField (Class|PlayFabJsonObject|GetObjectField _loginentity "Entity") "Id"))
    (else
      (return ""))))