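; Authentication actor that logs the player into PlayFab with an email address and password.
; LoginSuccessed caches the PlayFab ID, entity and authentication context from the result, then passes them to the PlayFabGameInstance as the login session.
; It then broadcasts OnLoginSuccessed, though a failed game instance cast skips only the session hand-off.
; IsLoggingIn reports whether a valid login context is stored.
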(event Custom|Login%20with%20Email
  (params (Email :type String) (Password :type String))
  (|LoginwithEmailAddress (Utilities|Struct|MakeClientLoginWithEmailAddressRequest 0 Email 0 Password) (EventDispatchers|CreateEvent :!event LoginSuccessed) (EventDispatchers|CreateEvent :!event PlayFapError)))

(fn ConstructionScript)

(fn IsLoggingin
  (return (Utilities|IsValid (Class|PlayFabBaseActor|GetLoginContext))))

(fn LoginSuccessed
  (params (result :type Client%20Login%20Result%20Structure) (customData :type Object%20Object%20Reference))
  (bind (_entitytoken _inforesultpayload _lastlogintime _newlycreated _playfabid _sessionticket _settingsforuser _treatmentassignment _authenticationcontext) (Utilities|Struct|BreakClientLoginResult result))
  (LocalVariables|SetPlayerEntity (Class|PlayFabJsonObject|GetObjectField _entitytoken "Entity"))
  (LocalVariables|SetPlayFabId _playfabid)
  (LocalVariables|SetLoginContext _authenticationcontext)
  (Utilities|FlowControl|Sequence
    (:then_0
      (bind _asplay_fab_game_instance (Utilities|Casting|CastToPlayFabGameInstance (Game|GetGameInstance)))
      (Class|PlayFabGameInstance|SetPlayFabLoginSession _asplay_fab_game_instance (LocalVariables|GetPlayFabId) (LocalVariables|GetPlayerEntity) (LocalVariables|GetLoginContext)))
    (:then_1
      (Default|CallOnLoginSuccessed))))