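; Actor that runs PlayFab multiplayer matchmaking, from ticket creation to handing over a game server address.
; It creates a ticket carrying the player entity and region latencies, stores the target map on the game instance, then polls status on a looping timer.
; A match yields the server's IP and port, or localhost as fallback, passed to OnMatchJoined with the PlayFab ID and pawn class read from user data.
; Cancellation clears the timer.
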(event Custom|Fetch%20Character%20Info
  (|GetUserData (Utilities|Struct|MakeClientGetUserDataRequest 0 "" (Class|PlayFabBaseActor|GetPlayFabId) (Class|PlayFabBaseActor|GetLoginContext)) (delegate Custom|GetUserDataSuccess) (EventDispatchers|CreateEvent :!event PlayFapError)))

(event Custom|GetUserDataSuccess
  (params (result :type Client%20Get%20User%20Data%20Result%20Structure) (customData :type Object%20Object%20Reference))
  (Variables|Default|SetPawnClass (Class|PlayFabJsonObject|GetStringField (Class|PlayFabJsonObject|GetObjectField (.Data (Utilities|Struct|BreakClientGetUserDataResult result)) "PawnClass") "Value")))

(event Custom|Create%20Matchmaking%20Ticket
  (params (QueueName :type String) (TargetMap :type String))
  (Utilities|FlowControl|Sequence
    (:then_0
      (bind _output_get (Variables|Default|SetMatchQueueName QueueName))
      (|MatchmakingTicket (Utilities|Struct|MakeMultiplayerCreateMatchmakingTicketRequest (CallFunction|ConstructTicketCreator) 0 (Variables|Default|GetTicketTimeout) 0 _output_get (Class|PlayFabBaseActor|GetLoginContext)) (delegate Custom|Create%20Matchmaking%20Ticket%20Successed) (EventDispatchers|CreateEvent :!event PlayFapError)))
    (:then_1
      (bind _asplay_fab_game_instance (Utilities|Casting|CastToPlayFabGameInstance (Game|GetGameInstance)))
      (Variables|/Script/PlayFabMultiplayer.PlayFabGameInstance|SetTravelTargetMap _asplay_fab_game_instance TargetMap))))

(event Custom|Create%20Matchmaking%20Ticket%20Successed
  (params (result :type Multiplayer%20Create%20Matchmaking%20Ticket%20Result%20Structure) (customData :type Object%20Object%20Reference))
  (Variables|Default|SetMatchTicketId (.TicketId (Utilities|Struct|BreakMultiplayerCreateMatchmakingTicketResult result)))
  (bind _returnvalue (Utilities|Time|SetTimerbyEvent (delegate Custom|Get%20Matchmaking%20Ticket) 7.0 true 3.0))
  (Variables|Default|SetMatchTicketTimeHanđle _returnvalue))

(event Custom|Get%20Matchmaking%20Ticket
  (|GetMatchmakingTicket (Utilities|Struct|MakeMultiplayerGetMatchmakingTicketRequest 0 false (Variables|Default|GetMatchQueueName) (Variables|Default|GetMatchTicketId) (Class|PlayFabBaseActor|GetLoginContext)) (delegate Custom|Get%20Matchmaking%20Ticket%20Successed) (EventDispatchers|CreateEvent :!event PlayFapError)))

(event Custom|Cancel%20Matchmaking%20Ticket
  (|CancelMatchmakingTicket (Utilities|Struct|MakeMultiplayerCancelMatchmakingTicketRequest 0 (Variables|Default|GetMatchQueueName) (Variables|Default|GetMatchTicketId) (Class|PlayFabBaseActor|GetLoginContext)) (delegate Custom|Cancel%20Matchmaking%20Ticket%20Successed) (EventDispatchers|CreateEvent :!event PlayFapError)
    (:then
      (Utilities|Time|ClearandInvalidateTimerbyHandle (Variables|Default|GetMatchTicketTimeHanđle)))))

(event Custom|Get%20Matchmaking%20Ticket%20Successed
  (params (result :type Multiplayer%20Get%20Matchmaking%20Ticket%20Result%20Structure) (customData :type Object%20Object%20Reference))
  (bind (_cancellationreasonstring _changenumber _created _creator _giveupafterseconds _matchid _members _memberstomatchwith _queuename _status) (Utilities|Struct|BreakMultiplayerGetMatchmakingTicketResult result))
  (Development|PrintString _status)
  (switch string _status
    (:Matched
      (|GetMatch (Utilities|Struct|MakeMultiplayerGetMatchRequest 0 false _matchid (Variables|Default|GetMatchQueueName) false (Class|PlayFabBaseActor|GetLoginContext)) (delegate Custom|Get%20Match%20Successed) (EventDispatchers|CreateEvent :!event PlayFapError)
        (:then
          _)))
    (:Canceled
      (Default|CallOnTicketCancelled)))
  (Utilities|Time|ClearandInvalidateTimerbyHandle (Variables|Default|GetMatchTicketTimeHanđle)))

(event Custom|Get%20Match%20Successed
  (params (result :type Multiplayer%20Get%20Match%20Result%20Structure) (customData :type Object%20Object%20Reference))
  (bind _serverdetails (Utilities|Struct|BreakMultiplayerGetMatchResult result))
  (if (Utilities|IsValid _serverdetails)
    (bind _returnvalue (Class|PlayFabJsonObject|GetObjectArrayField _serverdetails "Ports"))
    (Default|CallOnMatchJoined (Utilities|String|Append (Class|PlayFabJsonObject|GetStringField _serverdetails "IPV4Address") ":" (Utilities|String|ToString(Integer) (Math|Float|Truncate (Class|PlayFabJsonObject|GetNumberField (Utilities|Array|Get(acopy) _returnvalue) "Num")))) (Class|PlayFabBaseActor|GetPlayFabId) (Variables|Default|GetPawnClass))
    (else
      (Default|CallOnMatchJoined "127.0.0.1:7777" (Class|PlayFabBaseActor|GetPlayFabId) (Variables|Default|GetPawnClass)))))

(event Custom|Cancel%20Matchmaking%20Ticket%20Successed
  (params (result :type Multiplayer%20Cancel%20Matchmaking%20Ticket%20Result%20Structure) (customData :type Object%20Object%20Reference)))

(fn ConstructionScript)

(fn ConstructTicketCreator
  (for _array_element (Variables|Default|GetRegionLatencies)
    (bind _output_get (LocalVariables|SetLatency (Class|PlayFabJsonObject|ConstructJsonObject)))
    (Class|PlayFabJsonObject|SetStringField _output_get "Region" (.Region (Utilities|Struct|BreakRegionLatency _array_element)))
    (Class|PlayFabJsonObject|SetNumberField _output_get "Latency" (.Latency (Utilities|Struct|BreakRegionLatency _array_element)))
    (Utilities|Array|Add (LocalVariables|GetLatencies) _output_get))
  (bind _output_get_2 (LocalVariables|SetCreator (Class|PlayFabJsonObject|ConstructJsonObject)))
  (Class|PlayFabJsonObject|DecodeJson _output_get_2 "{ 
	\"Attributes\": 
	{ 
		\"DataObject\": {} 
	} 
}")
  (Class|PlayFabJsonObject|SetObjectField (LocalVariables|GetCreator) "Entity" (Class|PlayFabBaseActor|GetPlayFabEntity))
  (Class|PlayFabJsonObject|SetObjectArrayField (Class|PlayFabJsonObject|GetObjectField (Class|PlayFabJsonObject|GetObjectField (LocalVariables|GetCreator) "Attributes") "DataObject") "Latencies" (LocalVariables|GetLatencies))
  (return (LocalVariables|GetCreator)))