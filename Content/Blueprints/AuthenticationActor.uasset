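; Actor that handles PlayFab email/password login and exposes the resulting player session.
; On BeginPlay it restores the entity, auth context and PlayFab ID cached in PlayFabGameInstance.
; A successful login handler updates these values, saves them back to the game instance and fires an OnLoginSuccessed notification.
; Helpers report login state from auth context validity and read the player's entity ID.
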(event Custom|Login%20with%20Email
  (params (Email :type String) (Password :type String))
  (|LoginwithEmailAddress (Utilities|Struct|MakeClientLoginWithEmailAddressRequest 0 Email 0 Password (Variables|Default|GetAuthContext)) (EventDispatchers|CreateEvent :!event LoginSuccessed) (EventDispatchers|CreateEvent :!event PlayFapError)))

(event EventBeginPlay
  (bind _asplay_fab_game_instance (Utilities|Casting|CastToPlayFabGameInstance (Game|GetGameInstance)))
  (Variables|Default|SetPlayerEntity (Variables|/Script/PlayFabMultiplayer.PlayFabGameInstance|GetPlayFabEntity _asplay_fab_game_instance))
  (Variables|Default|SetAuthContext (Variables|/Script/PlayFabMultiplayer.PlayFabGameInstance|GetPlayFabLoginContext _asplay_fab_game_instance))
  (Variables|Default|SetPlayFabId (Variables|/Script/PlayFabMultiplayer.PlayFabGameInstance|GetPlayFabId _asplay_fab_game_instance)))

(fn ConstructionScript)

(fn IsLoggingin
  (return (Utilities|IsValid (Variables|Default|GetAuthContext))))

(fn LoginSuccessed
  (params (result :type Client%20Login%20Result%20Structure) (customData :type Object%20Object%20Reference))
  (bind (_entitytoken _inforesultpayload _lastlogintime _newlycreated _playfabid _sessionticket _settingsforuser _treatmentassignment _authenticationcontext) (Utilities|Struct|BreakClientLoginResult result))
  (Variables|Default|SetPlayerEntity (Class|PlayFabJsonObject|GetObjectField _entitytoken "Entity"))
  (Variables|Default|SetPlayFabId _playfabid)
  (Variables|Default|SetAuthContext _authenticationcontext)
  (Utilities|FlowControl|Sequence
    (:then_0
      (bind _asplay_fab_game_instance (Utilities|Casting|CastToPlayFabGameInstance (Game|GetGameInstance)))
      (Class|PlayFabGameInstance|SetPlayFabLoginSession _asplay_fab_game_instance (Variables|Default|GetPlayFabId) (Variables|Default|GetPlayerEntity) (Variables|Default|GetAuthContext)))
    (:then_1
      (Default|CallOnLoginSuccessed))))

(fn GetPlayerId
  (bind _playerentity (Variables|Default|GetPlayerEntity))
  (if (and (Utilities|IsValid _playerentity) (Class|PlayFabJsonObject|HasField _playerentity "Entity"))
    (return (Class|PlayFabJsonObject|GetStringField (Class|PlayFabJsonObject|GetObjectField _playerentity "Entity") "Id"))
    (else
      (return ""))))