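; BP_PlayFabCharacter queries PlayFab for the logged-in player's characters and prints them for inspection.
; ListCatalogCharacters calls GetAllUsersCharacters with the login PlayFab ID and context, then prints each returned character as JSON.
; A second request for the "character" catalog, with a callback printing each item, is present but never runs, so despite the event's name no catalog is fetched.
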(event Custom|List%20Catalog%20Characters
  (|GetAllUsersCharacters (Utilities|Struct|MakeClientListUsersCharactersRequest (Class|PlayFabBaseActor|GetLoginPlayFabId) (Class|PlayFabBaseActor|GetLoginContext)) (delegate Custom|CustomEvent_0) (EventDispatchers|CreateEvent :!event PlayFapError)))

(event Custom|CustomEvent_0
  (params (result :type Client%20List%20Users%20Characters%20Result%20Structure) (customData :type Object%20Object%20Reference))
  (for _array_element (.Characters (Utilities|Struct|BreakClientListUsersCharactersResult result))
    (Development|PrintString (Class|PlayFabJsonObject|EncodeJson _array_element))))

(event Custom|CustomEvent_1
  (params (result :type Client%20Get%20Catalog%20Items%20Result%20Structure) (customData :type Object%20Object%20Reference))
  (for _array_element (.Catalog (Utilities|Struct|BreakClientGetCatalogItemsResult result))
    (Development|PrintString (Utilities|String|ToString(Object) _array_element))))

(fn ConstructionScript)