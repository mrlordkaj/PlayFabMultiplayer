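; PlayFab matchmaking actor that creates and cancels queue tickets and resolves a match to a server address.
; Tickets use the LoginActor's credentials and entity, with per-region latencies packed into JSON creator attributes.
; A looping timer polls ticket status until matched or canceled, then a match fetches its details.
; OnMatchJoined broadcasts IP:port, falling back to localhost without server details, and PlayFabError broadcasts formatted errors through OnErrorMessage.
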(event Custom|Create%20Matchmaking%20Ticket
  (params (GiveUpAfterSeconds :type Integer) (QueueName :type String))
  (bind _output_get (Variables|Default|SetMatchQueueName QueueName))
  (|MatchmakingTicket (Utilities|Struct|MakeMultiplayerCreateMatchmakingTicketRequest (CallFunction|GetTicketCreator) 0 GiveUpAfterSeconds 0 _output_get (Variables|/PlayFabMultiplayer/Blueprints/PlayFabLoginActor.PlayFabLoginActor_C|GetLoginContext (Variables|Default|GetLoginActor))) (delegate Custom|Create%20Matchmaking%20Ticket%20Successed) (EventDispatchers|CreateEvent :!event PlayfabError)))

(event Custom|Create%20Matchmaking%20Ticket%20Successed
  (params (result :type Multiplayer%20Create%20Matchmaking%20Ticket%20Result%20Structure) (customData :type Object%20Object%20Reference))
  (Variables|Default|SetMatchTicketId (.TicketId (Utilities|Struct|BreakMultiplayerCreateMatchmakingTicketResult result)))
  (bind _returnvalue (Utilities|Time|SetTimerbyEvent (delegate Custom|Get%20Matchmaking%20Ticket) 1e+01 true))
  (Variables|Default|SetMatchTicketTimeHanđle _returnvalue))

(event Custom|Get%20Matchmaking%20Ticket
  (|GetMatchmakingTicket (Utilities|Struct|MakeMultiplayerGetMatchmakingTicketRequest 0 false (Variables|Default|GetMatchQueueName) (Variables|Default|GetMatchTicketId) (Variables|/PlayFabMultiplayer/Blueprints/PlayFabLoginActor.PlayFabLoginActor_C|GetLoginContext (Variables|Default|GetLoginActor))) (delegate Custom|Get%20Matchmaking%20Ticket%20Successed) (EventDispatchers|CreateEvent :!event PlayfabError)))

(event Custom|Cancel%20Matchmaking%20Ticket
  (|CancelMatchmakingTicket (Utilities|Struct|MakeMultiplayerCancelMatchmakingTicketRequest 0 (Variables|Default|GetMatchQueueName) (Variables|Default|GetMatchTicketId) (Variables|/PlayFabMultiplayer/Blueprints/PlayFabLoginActor.PlayFabLoginActor_C|GetLoginContext (Variables|Default|GetLoginActor))) (delegate Custom|Cancel%20Matchmaking%20Ticket%20Successed) (EventDispatchers|CreateEvent :!event PlayfabError)
    (:then
      (Utilities|Time|ClearandInvalidateTimerbyHandle (Variables|Default|GetMatchTicketTimeHanđle)))))

(event Custom|Get%20Matchmaking%20Ticket%20Successed
  (params (result :type Multiplayer%20Get%20Matchmaking%20Ticket%20Result%20Structure) (customData :type Object%20Object%20Reference))
  (bind (_cancellationreasonstring _changenumber _created _creator _giveupafterseconds _matchid _members _memberstomatchwith _queuename _status) (Utilities|Struct|BreakMultiplayerGetMatchmakingTicketResult result))
  (Development|PrintString _status)
  (switch string _status
    (:Matched
      (|GetMatch (Utilities|Struct|MakeMultiplayerGetMatchRequest 0 false _matchid (Variables|Default|GetMatchQueueName) false (Variables|/PlayFabMultiplayer/Blueprints/PlayFabLoginActor.PlayFabLoginActor_C|GetLoginContext (Variables|Default|GetLoginActor))) (delegate Custom|Get%20Match%20Successed) (EventDispatchers|CreateEvent :!event PlayfabError)
        (:then
          _)))
    (:Canceled
      _))
  (Utilities|Time|ClearandInvalidateTimerbyHandle (Variables|Default|GetMatchTicketTimeHanđle)))

(event Custom|Get%20Match%20Successed
  (params (result :type Multiplayer%20Get%20Match%20Result%20Structure) (customData :type Object%20Object%20Reference))
  (bind _serverdetails (Utilities|Struct|BreakMultiplayerGetMatchResult result))
  (if (Utilities|IsValid _serverdetails)
    (bind _returnvalue (Class|PlayFabJsonObject|GetObjectArrayField _serverdetails "Ports"))
    (Default|CallOnMatchJoined (Utilities|String|Append (Class|PlayFabJsonObject|GetStringField _serverdetails "IPV4Address") ":" (Utilities|String|ToString(Integer) (Math|Float|Truncate (Class|PlayFabJsonObject|GetNumberField (Utilities|Array|Get(acopy) _returnvalue) "Num")))))
    (else
      (Default|CallOnMatchJoined "127.0.0.1:7777"))))

(event Custom|Cancel%20Matchmaking%20Ticket%20Successed
  (params (result :type Multiplayer%20Cancel%20Matchmaking%20Ticket%20Result%20Structure) (customData :type Object%20Object%20Reference)))

(fn ConstructionScript)

(fn GetTicketCreator
  (for _array_element (Variables|Default|GetServerLatencies)
    (bind _output_get (LocalVariables|SetLatency (Class|PlayFabJsonObject|ConstructJsonObject)))
    (Class|PlayFabJsonObject|SetStringField _output_get "Region" (.Region (Utilities|Struct|BreakServerLatency _array_element)))
    (Class|PlayFabJsonObject|SetNumberField _output_get "Latency" (.Latency (Utilities|Struct|BreakServerLatency _array_element)))
    (Utilities|Array|Add (LocalVariables|GetLatencies) _output_get))
  (bind _output_get_2 (LocalVariables|SetCreator (Class|PlayFabJsonObject|ConstructJsonObject)))
  (Class|PlayFabJsonObject|DecodeJson _output_get_2 "{ 
	\"Entity\": null, 
	\"Attributes\": 
	{ 
		\"DataObject\": {} 
	} 
}")
  (Class|PlayFabJsonObject|MergeJsonObject (LocalVariables|GetCreator) (Variables|/PlayFabMultiplayer/Blueprints/PlayFabLoginActor.PlayFabLoginActor_C|GetLoginEntity (Variables|Default|GetLoginActor)) true)
  (Class|PlayFabJsonObject|SetObjectArrayField (Class|PlayFabJsonObject|GetObjectField (Class|PlayFabJsonObject|GetObjectField (LocalVariables|GetCreator) "Attributes") "DataObject") "Latencies" (LocalVariables|GetLatencies))
  (return (LocalVariables|GetCreator)))

(fn PlayFabError
  (params (error :type Play%20Fab%20Error%20Structure) (customData :type Object%20Object%20Reference))
  (bind (_haserror _errorcode _errorname _errormessage) (Utilities|Struct|BreakPlayFabError error))
  (bind _output_get (LocalVariables|SetMessage (Utilities|String|ToString(Text) (Utilities|Text|FormatText "{Message} ({Code})" _errormessage (Utilities|Text|ToText(Integer) _errorcode false false)))))
  (Development|PrintString _output_get true true "(R=1.000000,G=0.000000,B=0.000000,A=1.000000)")
  (Default|CallOnErrorMessage (LocalVariables|GetMessage)))