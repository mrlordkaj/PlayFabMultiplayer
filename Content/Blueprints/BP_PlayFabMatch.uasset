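; BP_PlayFabMatch is a PlayFab client Blueprint that fetches the player's character choice from user data.
; FetchCharacterInfo sends GetUserData with the current PlayFab ID and authentication context.
; Its success callback reads the Value string of the PawnClass field and stores it in PawnClass.
; Grant-character and register-user calls are left unwired, and Test is an empty stub.
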(event Custom|Fetch%20Character%20Info
  (|GetUserData (Utilities|Struct|MakeClientGetUserDataRequest 0 "" (Class|PlayFabBaseActor|GetPlayFabId) (Class|PlayFabBaseActor|GetAuthenticationContext)) (delegate Custom|GetUserDataSuccess) (EventDispatchers|CreateEvent :!event PlayFapError)))

(event Custom|GetUserDataSuccess
  (params (result :type Client%20Get%20User%20Data%20Result%20Structure) (customData :type Object%20Object%20Reference))
  (Variables|Default|SetPawnClass (Class|PlayFabJsonObject|GetStringField (Class|PlayFabJsonObject|GetObjectField (.Data (Utilities|Struct|BreakClientGetUserDataResult result)) "PawnClass") "Value")))

(event Custom|Test)

(event Custom|CustomEvent_2
  (params (result :type Client%20Grant%20Character%20to%20User%20Result%20Structure) (customData :type Object%20Object%20Reference)))

(fn ConstructionScript)